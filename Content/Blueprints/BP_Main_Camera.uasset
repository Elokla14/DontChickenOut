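; BP_Main_Camera is the main camera Blueprint, which tracks the player's chicken along the world Y axis.
; On BeginPlay it casts the player pawn to BP_Chicken and caches the reference.
; Each Tick it sets its location to the chicken's Y plus an offset, holding X and height fixed, with no interpolation or sweep.
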(event EventBeginPlay
  (bind _asbp_chicken (Utilities|Casting|CastToBP_Chicken (Game|Player|GetPlayerPawn 0)))
  (Variables|Default|SetChicken%20REF _asbp_chicken))

(event EventTick
  (params (DeltaSeconds :type Float%20%28single-precision%29))
  (Transformation|SetActorLocation (Math|Vector|MakeVector 0.0 (+ (.Y (Math|Vector|BreakVector (Transformation|GetActorLocation (Variables|Default|GetChicken%20REF)))) (Variables|Default|GetOffset%20Y)) 1.3e+03) false false))

(fn ConstructionScript)