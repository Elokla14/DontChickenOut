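; Lily pad platform that bounces and spins when the chicken is on it, using state and bounce animation defined outside this graph.
; BeginPlay picks a random yaw speed and has a random switch ahead of spawning a BP_Coin at the pad's location.
; Tick plays a 2D sound as a jump-on starts, runs the bounce animation, and rotates the pad while it carries the chicken.
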(event EventBeginPlay
  (|CallParentFunction)
  (Variables|Default|SetRotation (Math|Rotator|MakeRotator 0.0 0.0 (Math|Random|RandomFloatinRange -2e+01 2e+01)))
  (switch int (Math|Random|RandomInteger 3)
    (:0
      _)
    (:1
      _))
  (Game|SpawnActorfromClass "/Game/Blueprints/BP_Coin.BP_Coin_C" (Math|Transform|MakeTransform (Transformation|GetActorLocation)) "Undefined" 0 0))

(event EventTick
  (params (DeltaSeconds :type Float%20%28single-precision%29))
  (Variables|Default|SetMake%20Delta%20Seconds DeltaSeconds)
  (CallFunction|AttemptPlayJumpedonSound)
  (CallFunction|BouncingAnimation (Variables|Default|GetMake%20Delta%20Seconds))
  (if (Variables|Default|GetHas%20Chicken%20On%20Top)
    (Transformation|AddActorLocalRotation (* (Variables|Default|GetRotation) (Variables|Default|GetMake%20Delta%20Seconds)) false false)))

(fn ConstructionScript
  (|CallParentFunction))

(fn AttemptPlayJumpedonSound
  (if (and (== (Variables|Default|GetCurrent%20Jumped%20On%20Time) 0.0) (Variables|Default|GetIs%20Being%20Jumped%20On))
    (Audio|PlaySound2D "/Game/media/sounds/lily_pad.lily_pad" 1.0 1.0 0.0 0 0)))