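; Game mode for a Crossy Road-style chicken game that sets up camera and UI, procedurally builds the level and reloads it after game over.
; ConstructFloors spawns random grass, road, water and railroad chunks 20 rows ahead of the player, avoiding repeated types and shrinking maximum chunk length with progress.
; Shared clear-column positions link grass gaps to lily pads, while water rows limit same-direction log runs and require both directions between pad rows.
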(event EventBeginPlay
  (bind _returnvalue (Game|GetPlayerController 0))
  (CallFunction|CreateUI)
  (Input|EnableInput _returnvalue 0)
  (Variables|/Script/Engine.PlayerController|SetbShowMouseCursor _returnvalue true)
  (Variables|Default|SetCan%20Run%20Program true)
  (bind _outactors (Actor|GetAllActorswithTag "Camera"))
  (for _array_element _outactors
    (bind _asbp_main_camera (Utilities|Casting|CastToBP_Main_Camera _array_element))
    (bind _output_get (Variables|Default|SetCamera%20REF _asbp_main_camera))
    (Game|Player|SetViewTargetwithBlend (Game|GetPlayerController 0) _output_get 0.0 "VTBlend_Linear" 0.0 false)))

(event EventTick
  (params (DeltaSeconds :type Float%20%28single-precision%29))
  (if (Variables|Default|GetCan%20Run%20Program)
    (if (Variables|Default|GetConstructed%20Initial%20Floor%20Chunks)
      (if (Variables|Default|GetIs%20Game%20Over)
        (Variables|Default|SetIs%20Game%20Over false)
        (Utilities|FlowControl|Delay 3.0)
        (Game|OpenLevel(byName) "GamePlay"))
      (else
        (CallFunction|ConstructInitialFloors)
        (Variables|Default|SetConstructed%20Initial%20Floor%20Chunks true)))))

(fn ConstructionScript)

(fn CreateClearColumnPositions
  (bind _returnvalue (Math|Random|RandomInteger 8))
  (bind _returnvalue_2 (* _returnvalue 2e+02))
  (bind _returnvalue_3 (- _returnvalue_2 8e+02))
  (Variables|Default|SetClear%20Column%20Pos%20X1 -1.0)
  (Variables|Default|SetClear%20Column%20Pos%20X2 -1.0)
  (Variables|Default|SetClear%20Column%20Pos%20X3 -1.0)
  (for _index (range 0 (Math|Random|RandomInteger 2))
    (switch int _index
      (:0
        (Variables|Default|SetClear%20Column%20Pos%20X1 _returnvalue_3))
      (:1
        (Variables|Default|SetClear%20Column%20Pos%20X2 _returnvalue_3))
      (:2
        (Variables|Default|SetClear%20Column%20Pos%20X3 _returnvalue_3)))))

(fn CalcFloorSpawnY
  (return (- (* (Variables|Default|GetFloor%20Spawn%20Y%20Delta) (Math|Conversions|ToFloat(Integer) (Variables|Default|GetCurrent%20Floor%20Index))) 2e+02)))

(fn CreateGrassFloorChunk
  (params (Number%20of%20Floors :type Integer) (Center%20Clear%20Column :type Boolean))
  (if (== (Variables|Default|GetPrevious%20Floor%20Type%20Created) 2)
    _
    (else
      (CallFunction|CreateClearColumnPositions)))
  (if Center%20Clear%20Column
    (Variables|Default|SetClear%20Column%20Pos%20X3 0.0))
  (for _index (range 0 (- Number%20of%20Floors 1))
    (Variables|Default|SetCurrent%20Floor%20Index (+ (Variables|Default|GetCurrent%20Floor%20Index) 1))
    (bind _position_y (CallFunction|CalcFloorSpawnY))
    (Game|SpawnActorfromClass "/Game/Blueprints/BP_Grass.BP_Grass_C" (Math|Transform|MakeTransform (Math|Vector|MakeVector 0.0 _position_y 0.0)) "Undefined" 0 (not (== (Math|Integer|%(Integer) _index 2) 0)) (Variables|Default|GetClear%20Column%20Pos%20X1) (Variables|Default|GetClear%20Column%20Pos%20X2) (Variables|Default|GetClear%20Column%20Pos%20X3) (Variables|Default|GetChicken%20REF) _position_y 0)))

(fn CalcCurrentFloorTypetoCreate
  (Variables|Default|SetPrevious%20Floor%20Type%20Created (Variables|Default|GetCurrent%20Floor%20Type%20Created))
  (Variables|Default|SetCurrent%20Floor%20Type%20Created (Math|Random|RandomInteger 4))
  (if (== (Variables|Default|GetCurrent%20Floor%20Type%20Created) (Variables|Default|GetPrevious%20Floor%20Type%20Created))
    (switch int (Variables|Default|GetPrevious%20Floor%20Type%20Created)
      (:0
        (Variables|Default|SetCurrent%20Floor%20Type%20Created 1))
      (:1
        (Variables|Default|SetCurrent%20Floor%20Type%20Created 2))
      (:2
        (Variables|Default|SetCurrent%20Floor%20Type%20Created 3))
      (:3
        (Variables|Default|SetCurrent%20Floor%20Type%20Created 0)))))

(fn CreateRoadFloorChunk
  (params (Number%20Of%20Floors :type Integer))
  (for _index (range 0 (- Number%20Of%20Floors 1))
    (Variables|Default|SetCurrent%20Floor%20Index (+ (Variables|Default|GetCurrent%20Floor%20Index) 1))
    (bind _position_y (CallFunction|CalcFloorSpawnY))
    (Game|SpawnActorfromClass "/Game/Blueprints/BP_Road.BP_Road_C" (Math|Transform|MakeTransform (Math|Vector|MakeVector 0.0 _position_y 0.0)) "Undefined" 0 (>= _index 0) (Variables|Default|GetChicken%20REF) _position_y 0)))

(fn CreateRailroadFloorChunk
  (params (Number%20Of%20Floors :type Integer))
  (for _index (range 0 (- Number%20Of%20Floors 1))
    (Variables|Default|SetCurrent%20Floor%20Index (+ (Variables|Default|GetCurrent%20Floor%20Index) 1))
    (bind _position_y (CallFunction|CalcFloorSpawnY))
    (Game|SpawnActorfromClass "/Game/Blueprints/BP_Railroad.BP_Railroad_C" (Math|Transform|MakeTransform (Math|Vector|MakeVector 0.0 _position_y 0.0)) "Undefined" 0 (Variables|Default|GetChicken%20REF) _position_y 0)))

(fn CountNumberOfLillyPadstoCreate
  (Variables|Default|SetNumber%20Of%20Lilly%20Pads%20To%20Create 0)
  (if (!= (Variables|Default|GetClear%20Column%20Pos%20X1) -1.0)
    (Variables|Default|SetNumber%20Of%20Lilly%20Pads%20To%20Create (+ (Variables|Default|GetNumber%20Of%20Lilly%20Pads%20To%20Create) 1)))
  (if (!= (Variables|Default|GetClear%20Column%20Pos%20X2) -1.0)
    (Variables|Default|SetNumber%20Of%20Lilly%20Pads%20To%20Create (+ (Variables|Default|GetNumber%20Of%20Lilly%20Pads%20To%20Create) 1))
    (if (!= (Variables|Default|GetClear%20Column%20Pos%20X3) -1.0)
      (Variables|Default|SetNumber%20Of%20Lilly%20Pads%20To%20Create (+ (Variables|Default|GetNumber%20Of%20Lilly%20Pads%20To%20Create) 1)))))

(fn CreateWaterFloorChunk
  (params (Number%20Of%20Floors :type Integer))
  (for _index (range 0 (- Number%20Of%20Floors 1))
    (Variables|Default|SetCurrent%20Floor%20Index (+ (Variables|Default|GetCurrent%20Floor%20Index) 1))
    (bind _position_y (CallFunction|CalcFloorSpawnY))
    (if (== (Math|Random|RandomIntegerinRange 0 4) 0)
      (if (Variables|Default|GetCan%20Create%20Lilly%20Pads)
        ;[1 1 1] Can Create Lilly Pads
        (if (Variables|Default|GetCreated%20Lilly%20Pads%20Since%20Water%20Chunk%20Group%20Started)
          (CallFunction|CreateClearColumnPositions))
        (CallFunction|CountNumberOfLillyPadstoCreate)
        (Game|SpawnActorfromClass "/Game/Blueprints/BP_Water.BP_Water_C" (Math|Transform|MakeTransform (Math|Vector|MakeVector 0.0 _position_y 0.0)) "Undefined" 0 false false true (Variables|Default|GetNumber%20Of%20Lilly%20Pads%20To%20Create) (Variables|Default|GetClear%20Column%20Pos%20X1) (Variables|Default|GetClear%20Column%20Pos%20X2) (Variables|Default|GetClear%20Column%20Pos%20X3) (Variables|Default|GetChicken%20REF) _position_y 0)
        (Variables|Default|SetCreated%20Lilly%20Pads%20Since%20Water%20Chunk%20Group%20Started true)
        (Variables|Default|SetCan%20Create%20Lilly%20Pads false)
        (Variables|Default|SetCreated%20Left%20Logs%20Since%20Lilly%20Pads false)
        (Variables|Default|SetCreated%20Right%20Logs%20Since%20Lilly%20Pads false)
        (else
          ;[1 1 1] Can not create lilly pads
          (bind _output_get (Variables|Default|SetCreate%20Logs%20Left (Math|Random|RandomBool) :!label _label))
          (if (Math|Boolean|Equal(Boolean) _output_get (Variables|Default|GetPrevious%20Log%20Creation%20Direction))
            (bind _output_get_2 (Variables|Default|SetNumber%20Of%20Logs%20Created%20In%20Same%20Direction (+ (Variables|Default|GetNumber%20Of%20Logs%20Created%20In%20Same%20Direction) 1)))
            (if (> _output_get_2 2)
              (bind _output_get_3 (Variables|Default|SetCreate%20Logs%20Left (not (Variables|Default|GetCreate%20Logs%20Left))))
              (Variables|Default|SetNumber%20Of%20Logs%20Created%20In%20Same%20Direction 1)
              (Variables|Default|SetPrevious%20Log%20Creation%20Direction _output_get_3))
            (else
              (Variables|Default|SetNumber%20Of%20Logs%20Created%20In%20Same%20Direction 1)))
          (Game|SpawnActorfromClass "/Game/Blueprints/BP_Water.BP_Water_C" (Math|Transform|MakeTransform (Math|Vector|MakeVector 0.0 _position_y 0.0)) "Undefined" 0 true (Variables|Default|GetCreate%20Logs%20Left) false 0 (Variables|Default|GetClear%20Column%20Pos%20X1) (Variables|Default|GetClear%20Column%20Pos%20X2) (Variables|Default|GetClear%20Column%20Pos%20X3) (Variables|Default|GetChicken%20REF) _position_y 0)
          (if (Variables|Default|GetCreate%20Logs%20Left)
            (Variables|Default|SetCreated%20Left%20Logs%20Since%20Lilly%20Pads true)
            (else
              (Variables|Default|SetCreated%20Right%20Logs%20Since%20Lilly%20Pads true)))
          (if (Variables|Default|GetCreated%20Left%20Logs%20Since%20Lilly%20Pads)
            (if (Variables|Default|GetCreated%20Right%20Logs%20Since%20Lilly%20Pads)
              (Variables|Default|SetCan%20Create%20Lilly%20Pads true)))
          (Variables|Default|SetPrevious%20Log%20Creation%20Direction (Variables|Default|GetCreate%20Logs%20Left))))
      (else
        (goto _label)))))

(fn ConstructFloors
  (bind _number_of_chunks_explored_forward (Variables|Default|GetNumber%20Of%20Chunks%20Explored%20Forward))
  (bind _number_of_chunks_explored_forward_2 (Variables|Default|GetNumber%20Of%20Chunks%20Explored%20Forward))
  (bind _returnvalue (/ _number_of_chunks_explored_forward_2 20))
  (bind _returnvalue_2 (/ _number_of_chunks_explored_forward 20))
  (bind _returnvalue_3 (- 6 _returnvalue))
  (bind _returnvalue_4 (- 6 _returnvalue_2))
  (bind _returnvalue_5 (Math|Random|RandomInteger _returnvalue_3))
  (bind _returnvalue_6 (Math|Random|RandomInteger _returnvalue_4))
  (bind _returnvalue_7 (+ _returnvalue_6 1))
  (bind _returnvalue_8 (+ _returnvalue_5 1))
  (while (< (- (Variables|Default|GetCurrent%20Floor%20Index) (Variables|Default|GetPlayer%20Pos%20Index)) 20)
    (CallFunction|CalcCurrentFloorTypetoCreate)
    (switch int (Variables|Default|GetCurrent%20Floor%20Type%20Created)
      (:0
        (if (< _returnvalue_8 1)
          (CallFunction|CreateGrassFloorChunk _returnvalue_8 false)
          (else
            (CallFunction|CreateGrassFloorChunk 1 false))))
      (:1
        (CallFunction|CreateRoadFloorChunk _returnvalue_7))
      (:2
        (Variables|Default|SetCreated%20Lilly%20Pads%20Since%20Water%20Chunk%20Group%20Started false)
        (CallFunction|CreateWaterFloorChunk _returnvalue_7))
      (:3
        (CallFunction|CreateRailroadFloorChunk _returnvalue_7)))))

(fn ConstructInitialFloors
  (CallFunction|CreateGrassFloorChunk 8 false)
  (CallFunction|CreateGrassFloorChunk 2 true)
  (CallFunction|ConstructFloors))

(fn CreateUI
  (bind _returnvalue (UserInterface|CreateWidget "/Game/UI/UI_GamePlay.UI_GamePlay_C"))
  (Variables|/Game/UI/UI_GamePlay.UI_GamePlay_C|SetGame%20Mode%20Ref _returnvalue self)
  (UserInterface|Viewport|AddtoViewport _returnvalue 0))